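; Game State Blueprint for BomberGuys, apparently meant to sync player info across clients, but currently mostly scaffolding.
; Its custom update and name-set events are empty, and its player-listing and debug-drawing nodes are disconnected.
; The PlayerNames RepNotify loops over every BP_BomberGuy without acting, as the player-info widget refresh is unwired.
; The Player Array RepNotify only prints a debug string.
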(event Custom|UpdateGameState)

(event Custom|When%20playerNameSet)

(event Custom|GS_Update)

(fn ConstructionScript)

(fn OnRepPlayerNames
  (bind _outactors (Actor|GetAllActorsOfClass "/bomber-guys/Blueprints/BP_BomberGuy.BP_BomberGuy_C"))
  (for _array_element _outactors
    _))

(fn OnRepPlayerArray
  (Development|PrintString "REP NOTIFY"))