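; BP_Distrabctable is a destructible wall that can drop a bonus pickup when destroyed, apparently for a Bomberman-style game.
; S_DistroyWall, also reached from DestroyKillPers after a short delay, sets IsDistroyed, whose RepNotify removes the cube and triggers bonus spawning.
; S_SpawnBonus usually spawns either a leg or fire bonus at the wall's location.
; Branches for other bonuses and debuffs are disconnected and never run.
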(event Custom|DestroyKillPers
  (Utilities|FlowControl|Delay 0.1)
  (CallFunction|SDistroyWall))

(event Custom|S_DistroyWall
  (Variables|Default|SetisDistroyed true))

(event Custom|S_SpawnBonus
  (Development|PrintString "spawn bonus")
  (if (Math|Random|RandomBoolwithWeight 0.8)
    (switch int (Math|Random|RandomIntegerinRange 0 1)
      (:0
        ;[0.3588 1 0.03754] Comment
        ;;[0.09295 0.7969 0.008825] Пинаножка
        (Utilities|SpawnBonus "/bomber-guys/Blueprints/Bonuses/GoodBonuses/BP_Bonus_Leg.BP_Bonus_Leg_C"))
      (:1
        ;;[0.09295 0.7969 0.008825] Огонь + 1
        (Utilities|SpawnBonus "/bomber-guys/Blueprints/Bonuses/GoodBonuses/BP_Bonus_Fire.BP_Bonus_Fire_C")))))

(event Custom|Distraction
  (Development|PrintString "distroy")
  (CallFunction|SSpawnBonus))

(fn ConstructionScript)

(fn OnRepIsDistroyed
  (Components|DestroyComponent (Variables|Default|GetCube))
  (CallFunction|Distraction))