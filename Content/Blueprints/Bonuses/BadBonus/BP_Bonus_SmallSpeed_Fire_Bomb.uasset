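; A bad-bonus actor that temporarily debuffs the player's BP_BomberGuy, cutting bomb time, fire length and walk speed.
; On BeginPlay it casts player character 0 and applies the reduced values immediately, with no pickup logic in its graphs.
; After a ten-second delay it writes back hardcoded normal values, rather than the player's previous stats, and destroys itself.
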(event EventBeginPlay
  ;[0.7969 0 0] Comment
  (bind _asbp_bomber_guy (Utilities|Casting|CastToBP_BomberGuy (Game|GetPlayerCharacter 0)))
  (Variables|/bomber-guys/Blueprints/BP_BomberGuy.BP_BomberGuy_C|SetBombTime _asbp_bomber_guy 1.0)
  (Variables|/bomber-guys/Blueprints/BP_BomberGuy.BP_BomberGuy_C|SetLengthOfFire _asbp_bomber_guy 1.0)
  (Variables|/Script/Engine.CharacterMovementComponent|SetMaxWalkSpeed (Variables|/Script/Engine.Character|GetCharacterMovement _asbp_bomber_guy) 2.5e+02)
  (Utilities|FlowControl|Delay 1e+01)
  (Variables|/bomber-guys/Blueprints/BP_BomberGuy.BP_BomberGuy_C|SetBombTime _asbp_bomber_guy 3.0)
  (Variables|/bomber-guys/Blueprints/BP_BomberGuy.BP_BomberGuy_C|SetLengthOfFire _asbp_bomber_guy 2.0)
  (Variables|/Script/Engine.CharacterMovementComponent|SetMaxWalkSpeed (Variables|/Script/Engine.Character|GetCharacterMovement _asbp_bomber_guy) 4e+02)
  (Actor|DestroyActor))

(fn ConstructionScript)