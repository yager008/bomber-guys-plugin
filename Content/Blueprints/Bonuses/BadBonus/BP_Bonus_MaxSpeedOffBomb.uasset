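; BP_Bonus_MaxSpeedOffBomb is a timed "bad bonus" effect actor that makes the player fast and invisible while hampering bomb use.
; On BeginPlay it casts player 0 to BP_BomberGuy, raises BombTime and walk speed, and hides the character.
; After a ten-second Delay it writes back hardcoded defaults rather than saved values, unhides the character and destroys itself.
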(event EventBeginPlay
  ;[0.7969 0 0] Отключение бомб, скорость 1000
  (bind _asbp_bomber_guy (Utilities|Casting|CastToBP_BomberGuy (Game|GetPlayerCharacter 0)))
  (Variables|/bomber-guys/Blueprints/BP_BomberGuy.BP_BomberGuy_C|SetBombTime _asbp_bomber_guy 1e+01)
  (Variables|/Script/Engine.CharacterMovementComponent|SetMaxWalkSpeed (Variables|/Script/Engine.Character|GetCharacterMovement _asbp_bomber_guy) 1e+03)
  (Rendering|SetActorHiddenInGame _asbp_bomber_guy true)
  (Utilities|FlowControl|Delay 1e+01)
  (Variables|/bomber-guys/Blueprints/BP_BomberGuy.BP_BomberGuy_C|SetBombTime _asbp_bomber_guy 3.0)
  (Variables|/Script/Engine.CharacterMovementComponent|SetMaxWalkSpeed (Variables|/Script/Engine.Character|GetCharacterMovement _asbp_bomber_guy) 4e+02)
  (Rendering|SetActorHiddenInGame _asbp_bomber_guy false)
  (Actor|DestroyActor))

(fn ConstructionScript)