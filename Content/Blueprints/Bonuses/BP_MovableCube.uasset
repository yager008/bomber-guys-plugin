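; A cube that BP_BomberGuy pushes around the level by overlapping one of its four directional trigger components.
; Each overlap sets that direction's flag, cleared on exit, and Tick calls MoveCube for all four directions after a tiny Delay.
; MoveCube line-traces along the direction's arrow and, while the flag is set, steps the cube forward without sweep unless a hit lies within a short distance.
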(event OnComponentBeginOverlap(Right)
  (params (OverlappedComponent :type Primitive%20Component%20Object%20Reference) (OtherActor :type Actor%20Object%20Reference) (OtherComp :type Primitive%20Component%20Object%20Reference) (OtherBodyIndex :type Integer) (bFromSweep :type Boolean) (SweepResult :type Hit%20Result%20Structure%20%28by%20ref%29))
  ;[1 0.704 0 0.634] Comment
  (Utilities|Casting|CastToBP_BomberGuy OtherActor)
  (Variables|Default|SetRight_ true))

(event OnComponentEndOverlap(Right)
  (params (OverlappedComponent :type Primitive%20Component%20Object%20Reference) (OtherActor :type Actor%20Object%20Reference) (OtherComp :type Primitive%20Component%20Object%20Reference) (OtherBodyIndex :type Integer))
  ;[1 0.704 0 0.634] Comment
  (Utilities|Casting|CastToBP_BomberGuy OtherActor)
  (Variables|Default|SetRight_ false))

(event OnComponentBeginOverlap(Left)
  (params (OverlappedComponent :type Primitive%20Component%20Object%20Reference) (OtherActor :type Actor%20Object%20Reference) (OtherComp :type Primitive%20Component%20Object%20Reference) (OtherBodyIndex :type Integer) (bFromSweep :type Boolean) (SweepResult :type Hit%20Result%20Structure%20%28by%20ref%29))
  ;[1 0.704 0 0.634] Comment
  (Utilities|Casting|CastToBP_BomberGuy OtherActor)
  (Variables|Default|SetLeft_ true))

(event OnComponentEndOverlap(Left)
  (params (OverlappedComponent :type Primitive%20Component%20Object%20Reference) (OtherActor :type Actor%20Object%20Reference) (OtherComp :type Primitive%20Component%20Object%20Reference) (OtherBodyIndex :type Integer))
  ;[1 0.704 0 0.634] Comment
  (Utilities|Casting|CastToBP_BomberGuy OtherActor)
  (Variables|Default|SetLeft_ false))

(event OnComponentBeginOverlap(Up)
  (params (OverlappedComponent :type Primitive%20Component%20Object%20Reference) (OtherActor :type Actor%20Object%20Reference) (OtherComp :type Primitive%20Component%20Object%20Reference) (OtherBodyIndex :type Integer) (bFromSweep :type Boolean) (SweepResult :type Hit%20Result%20Structure%20%28by%20ref%29))
  ;[1 0.704 0 0.634] Comment
  (Utilities|Casting|CastToBP_BomberGuy OtherActor)
  (Variables|Default|SetUp_ true))

(event OnComponentEndOverlap(Up)
  (params (OverlappedComponent :type Primitive%20Component%20Object%20Reference) (OtherActor :type Actor%20Object%20Reference) (OtherComp :type Primitive%20Component%20Object%20Reference) (OtherBodyIndex :type Integer))
  ;[1 0.704 0 0.634] Comment
  (Utilities|Casting|CastToBP_BomberGuy OtherActor)
  (Variables|Default|SetUp_ false))

(event OnComponentBeginOverlap(down)
  (params (OverlappedComponent :type Primitive%20Component%20Object%20Reference) (OtherActor :type Actor%20Object%20Reference) (OtherComp :type Primitive%20Component%20Object%20Reference) (OtherBodyIndex :type Integer) (bFromSweep :type Boolean) (SweepResult :type Hit%20Result%20Structure%20%28by%20ref%29))
  ;[1 0.704 0 0.634] Comment
  (Utilities|Casting|CastToBP_BomberGuy OtherActor)
  (Variables|Default|SetDown_ true))

(event OnComponentEndOverlap(down)
  (params (OverlappedComponent :type Primitive%20Component%20Object%20Reference) (OtherActor :type Actor%20Object%20Reference) (OtherComp :type Primitive%20Component%20Object%20Reference) (OtherBodyIndex :type Integer))
  ;[1 0.704 0 0.634] Comment
  (Utilities|Casting|CastToBP_BomberGuy OtherActor)
  (Variables|Default|SetDown_ false))

(event EventTick
  (params (DeltaSeconds :type Float%20%28single-precision%29))
  ;[0.5567 1 0 0.377] Comment
  (Utilities|FlowControl|Delay 0.001)
  (Utilities|FlowControl|Sequence
    (:then_0
      (Utilities|MoveCube (Variables|Default|GetLeft_) (Variables|Default|GetLestArrow)))
    (:then_1
      (Utilities|MoveCube (Variables|Default|GetRight_) (Variables|Default|GetRightArrow)))
    (:then_2
      (Utilities|MoveCube (Variables|Default|GetUp_) (Variables|Default|GetUpArrow)))
    (:then_3
      (Utilities|MoveCube (Variables|Default|GetDown_) (Variables|Default|GetDownArrow)))))

(fn ConstructionScript)