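; Bomberman-style bomb that explodes after a fuse delay, or sooner through FireBomb.
; The blast line-traces four ways from its grid-snapped cell, spawning staggered explosion emitters up to the fire length plus a collision box per direction.
; Sphere collision switches on once a BomberGuy leaves the overlap.
; A hit from a player with the kick bonus slides it via timeline-driven S_/M_ events until a forward trace finds an obstacle.
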(event OnComponentEndOverlap(CollShper)
  (params (OverlappedComponent :type Primitive%20Component%20Object%20Reference) (OtherActor :type Actor%20Object%20Reference) (OtherComp :type Primitive%20Component%20Object%20Reference) (OtherBodyIndex :type Integer))
  ;[1 0.8387 0.2705 0.597] Коллизия снарядов
  (Utilities|Casting|CastToBP_BomberGuy OtherActor)
  (Collision|SetCollisionEnabled (Variables|Default|GetSphere) "QueryAndPhysics"))

(event Custom|FireBomb
  (bind _returnvalue (Transformation|GetActorLocation))
  (bind _self self)
  (bind _returnvalue_2 (Class|KismetMathLibrary|VectorSnappedtoGrid _returnvalue 1e+02))
  (bind _returnvalue_3 (Math|Conversions|ToTransform(Vector) _returnvalue_2))
  (bind (_x _y _z) (Math|Vector|BreakVector (.location _returnvalue_3)))
  ;[0.5193 1 0 0.528] взрыв
  (Utilities|FlowControl|Delay 0.1)
  (Effects|SpawnEmitteratLocation 0 (Math|Vector|MakeVector _x _y (- _z 0.0)) "0, 0, 0" "0.800000,0.800000,0.800000")
  (Utilities|BombVzr)
  (Utilities|LocationSnar (.location _returnvalue_3) "NewEnumerator0")
  (Utilities|LocationSnar (.location _returnvalue_3) "NewEnumerator1")
  (Utilities|LocationSnar (.location _returnvalue_3) "NewEnumerator2")
  (Utilities|LocationSnar (.location _returnvalue_3) "NewEnumerator3")
  (Utilities|IsValid _self
    (:Is%20Valid
      (Actor|DestroyActor _self))))

(event Custom|M_TickPinaLag
  ;[0.04167 1 0.4904 0.424] kick bomb bonus
  (Transformation|AddActorLocalOffset (* (Variables|Пинаножка|GetPushDirection) 3e+02 (Variables|Пинаножка|GetDelta%20Seconds)) false false))

(event Custom|S_TickPinaLag
  ;[0.04167 1 0.4904 0.424] kick bomb bonus
  (CallFunction|MTickPinaLag))

(event EventBeginPlay
  (bind _returnvalue (Transformation|GetActorLocation))
  (bind _self self)
  (bind _returnvalue_2 (Class|KismetMathLibrary|VectorSnappedtoGrid _returnvalue 1e+02))
  (bind _returnvalue_3 (Math|Conversions|ToTransform(Vector) _returnvalue_2))
  (bind (_x _y _z) (Math|Vector|BreakVector (.location _returnvalue_3)))
  ;[0.5193 1 0 0.528] взрыв
  (Rendering|Material|SetMaterial (Variables|Default|GetSphere) 0 (Variables|Default|GetMaterialBomb))
  ;;[1 1 1] Время до взрыват
  (Utilities|FlowControl|Delay (Variables|Default|GetTimeBomb))
  (Effects|SpawnEmitteratLocation 0 (Math|Vector|MakeVector _x _y (- _z 0.0)) "0, 0, 0" "0.800000,0.800000,0.800000")
  (Utilities|BombVzr)
  (Utilities|LocationSnar (.location _returnvalue_3) "NewEnumerator0")
  (Utilities|LocationSnar (.location _returnvalue_3) "NewEnumerator1")
  (Utilities|LocationSnar (.location _returnvalue_3) "NewEnumerator2")
  (Utilities|LocationSnar (.location _returnvalue_3) "NewEnumerator3")
  (Utilities|IsValid _self
    (:Is%20Valid
      (Actor|DestroyActor _self))))

(event Collision|EventHit
  (params (MyComp :type Primitive%20Component%20Object%20Reference) (Other :type Actor%20Object%20Reference) (OtherComp :type Primitive%20Component%20Object%20Reference) (bSelfMoved :type Boolean) (HitLocation :type Vector :default "0, 0, 0") (HitNormal :type Vector :default "0, 0, 0") (NormalImpulse :type Vector :default "0, 0, 0") (Hit :type Hit%20Result%20Structure%20%28by%20ref%29))
  (bind _returnvalue (Transformation|GetActorForwardVector Other))
  (bind _returnvalue_2 (Transformation|GetActorLocation))
  (bind _returnvalue_3 (Math|Float|Round (.y _returnvalue)))
  (bind _returnvalue_4 (Math|Float|Round (.x _returnvalue)))
  ;[0.04167 1 0.4904 0.424] kick bomb bonus
  (Variables|Пинаножка|SetPinaLags? true)
  (bind _asbp_bomber_guy (Utilities|Casting|CastToBP_BomberGuy Other))
  (if (Variables|/bomber-guys/Blueprints/BP_BomberGuy.BP_BomberGuy_C|GetBonus_Leg _asbp_bomber_guy)
    (Variables|Пинаножка|SetcanMove true)
    (Utilities|SoundPinaLaegs)
    (if (not (== (Math|Integer|Absolute(Integer) _returnvalue_4) (Math|Integer|Absolute(Integer) _returnvalue_3)))
      (Variables|Пинаножка|SetPushDirection (Math|Vector|MakeVector (Math|Conversions|ToFloat(Integer) _returnvalue_4) (Math|Conversions|ToFloat(Integer) _returnvalue_3) 0.0))
      (bind _returnvalue_5 (Collision|LineTraceByChannel _returnvalue_2 (+ _returnvalue_2 (* (Variables|Пинаножка|GetPushDirection) 55.0)) "TraceTypeQuery1" false 0 "None" true "(R=1.000000,G=0.820313,B=0.196835,A=1.000000)"))
      (if _returnvalue_5
        (Variables|Пинаножка|SetcanMove false)
        (Transformation|AddActorLocalOffset (* (Variables|Пинаножка|GetPushDirection) -3e+02 (Variables|Пинаножка|GetDelta%20Seconds)) false false)
        (Timeline|Timeline_1 Stop
          (:Update
            (if (Variables|Пинаножка|GetcanMove)
              (CallFunction|STickPinaLag))))))))

(event EventTick
  (params (DeltaSeconds :type Float%20%28single-precision%29))
  (bind _returnvalue (Transformation|GetActorLocation))
  ;[0.04167 1 0.4904 0.424] kick bomb bonus
  (if (Variables|Пинаножка|GetPinaLags?)
    (Utilities|FlowControl|Sequence
      (:then_0
        (Variables|Пинаножка|SetDelta%20Seconds DeltaSeconds)
        (if (Variables|Пинаножка|GetcanMove)
          (Timeline|Timeline_1 PlayFromStart
            (:Update
              (if (Variables|Пинаножка|GetcanMove)
                (CallFunction|STickPinaLag))))
          (else
            (Timeline|Timeline_1 Stop))))
      (:then_1
        (bind _returnvalue_2 (Collision|LineTraceByChannel _returnvalue (+ _returnvalue (* (Variables|Пинаножка|GetPushDirection) 55.0)) "TraceTypeQuery1" false 0 "None" true "(R=1.000000,G=0.820313,B=0.196835,A=1.000000)"))
        (if _returnvalue_2
          (Variables|Пинаножка|SetcanMove false)
          (Transformation|AddActorLocalOffset (* (Variables|Пинаножка|GetPushDirection) -3e+02 (Variables|Пинаножка|GetDelta%20Seconds)) false false)
          (Timeline|Timeline_1 Stop))))))

(fn ConstructionScript)

(fn NFire+
  (params (N_fire+ :type Float%20%28double-precision%29))
  (Variables|Спавнвзрыва|SetLengthOfFIre N_fire+)
  (return 0.0))

(fn NSn
  (params (N_Sn+ :type Integer))
  (return 0))