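; Moving hitbox for a bomb explosion that sweeps from Start to End on a Timeline lerp, then destroys itself.
; Overlaps destroy BP_Distrabctable actors, kill BP_BomberGuy players and chain-detonate any BP_Bomb other than its instigator.
; Kills of other players increment NumberOfKills on HeroBomberRef's PlayerState and notify that pawn, while self-kills earn no credit.
; Debug prints and a debug sphere remain in the kill path.
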(event OnComponentBeginOverlap(Box)
  (params (OverlappedComponent :type Primitive%20Component%20Object%20Reference) (OtherActor :type Actor%20Object%20Reference) (OtherComp :type Primitive%20Component%20Object%20Reference) (OtherBodyIndex :type Integer) (bFromSweep :type Boolean) (SweepResult :type Hit%20Result%20Structure%20%28by%20ref%29))
  (bind _herobomberref (Variables|Default|GetHeroBomberRef))
  ;[0.6987 0.4371 1 0.518] Comment
  (Variables|Default|SethitComponent OtherComp)
  (Variables|Default|SetHit%20Actor OtherActor)
  (bind _asbp_distrabctable (Utilities|Casting|CastToBP_Distrabctable (Variables|Default|GetHit%20Actor))
    (:then
      (Utilities|IsValid _asbp_distrabctable
        (:Is%20Valid
          (Default|DestroyKillPers _asbp_distrabctable))))
    (:CastFailed
      (bind _asbp_bomber_guy (Utilities|Casting|CastToBP_BomberGuy (Variables|Default|GetHit%20Actor))
        (:then
          (Development|PrintString "KIIIILLLL" true true "(R=0.796875,G=0.000000,B=0.000000,A=1.000000)")
          (Utilities|IsValid _asbp_bomber_guy
            (:Is%20Valid
              (Development|PrintString "Kill")
              (Utilities|IsValid (Pawn|GetController _asbp_bomber_guy)
                (:Is%20Valid
                  (Utilities|IsValid _herobomberref
                    (:Is%20Valid
                      (Rendering|Debug|DrawDebugSphere (Transformation|GetActorLocation _herobomberref) 3e+02 12 "(R=0.000000,G=0.004275,B=1.000000,A=1.000000)" 0.0 12.0)
                      (Utilities|FlowControl|Sequence
                        (:then_0
                          (if (!= (Variables|Default|GetHit%20Actor) (Variables|Default|GetHeroBomberRef))
                            (Utilities|IsValid (Variables|Default|GetHeroBomberRef)
                              (:Is%20Valid
                                (bind _asps_bomber_guys (Utilities|Casting|CastToPS_BomberGuys (Variables|/Script/Engine.Controller|GetPlayerState (Pawn|GetController (Variables|Default|GetHeroBomberRef)))))
                                (Math|Integer|IncrementInt (Variables|/bomber-guys/Blueprints/Core/PS_BomberGuys.PS_BomberGuys_C|GetnumberOfKills _asps_bomber_guys)
                                  (:%20%20
                                    (Development|PrintString (Utilities|String|Append (Variables|/bomber-guys/Blueprints/Core/PS_BomberGuys.PS_BomberGuys_C|GetPlayerName _asps_bomber_guys) "+" (Utilities|String|ToString(Integer) (Variables|/bomber-guys/Blueprints/Core/PS_BomberGuys.PS_BomberGuys_C|GetnumberOfKills _asps_bomber_guys))))
                                    (Default|PawnEnemyKillFunction (Variables|Default|GetHeroBomberRef))))))
                            (else
                              (Development|PrintString "SELF KILLLLLLLLLLLLL!"))))
                        (:then_1
                          (Default|Kill _asbp_bomber_guy (Pawn|GetController _asbp_bomber_guy)))))))))))
        (:CastFailed
          (bind _asbp_bomb (Utilities|Casting|CastToBP_Bomb (Variables|Default|GetHit%20Actor)))
          (if (not (== _asbp_bomb (Game|GetInstigator)))
            (Default|FireBomb _asbp_bomb)))))))

(event Custom|S_SetKills++
  (params (PlayerName :type String) (Target :type Controller%20Object%20Reference))
  (bind _asps_bomber_guys (Utilities|Casting|CastToPS_BomberGuys (Variables|/Script/Engine.Controller|GetPlayerState (Pawn|GetController (Variables|Default|GetHeroBomberRef)))))
  (Math|Integer|IncrementInt (Variables|/bomber-guys/Blueprints/Core/PS_BomberGuys.PS_BomberGuys_C|GetnumberOfKills _asps_bomber_guys)
    (:%20%20
      (Development|PrintString (Utilities|String|Append (Variables|/bomber-guys/Blueprints/Core/PS_BomberGuys.PS_BomberGuys_C|GetPlayerName _asps_bomber_guys) "+" (Utilities|String|ToString(Integer) (Variables|/bomber-guys/Blueprints/Core/PS_BomberGuys.PS_BomberGuys_C|GetnumberOfKills _asps_bomber_guys))))
      (Default|PawnEnemyKillFunction (Variables|Default|GetHeroBomberRef)))))

(event EventBeginPlay
  ;[0.1284 1 0.7889 0.356] Comment
  (bind _newtrack_0 (Timeline|Timeline PlayFromStart)
    (:Update
      (Transformation|SetActorLocation (Math|Vector|Lerp(Vector) (Variables|Default|GetStart) (Variables|Default|GetEnd) _newtrack_0) false false))
    (:Finished
      (Actor|DestroyActor))))

(event EventEndPlay
  (params (EndPlayReason :type EEndPlayReason%20Enum :default "Destroyed")))

(fn ConstructionScript)

(fn MTickPinaLag)

(fn SSetPlayerNameinPS
  (params (PlayerName1 :type String) (Target1 :type Controller%20Object%20Reference)))