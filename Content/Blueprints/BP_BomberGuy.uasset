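; Playable Bomberman-style robot character that drops grid-snapped bombs, toggles between fixed arena and first-person cameras, and can drive a second local player's pawn.
; Bombs are capped by a timed DoN and occupancy check, spawning locally then replicating through server and multicast events.
; GameInstance supplies player name to PlayerState and color to a RepNotify that swaps mesh and bomb material.
; It also handles pausing, debug HUD and death respawn via GameMode.
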(event Custom|update%20color
  ;[1 0.9373 0.0697] Character color change
  (bind _asgi_bomber_guys (Utilities|Casting|CastToGI_BomberGuys (Game|GetGameInstance)))
  (CallFunction|SSetHeroStyle (Variables|/bomber-guys/Blueprints/Core/GI_BomberGuys.GI_BomberGuys_C|GetPlayerEnum _asgi_bomber_guys)))

(event Custom|S_SetPlayerNameInPS
  (params (PlayerName :type String) (Target :type Controller%20Object%20Reference))
  (bind _asps_bomber_guys (Utilities|Casting|CastToPS_BomberGuys (Variables|/Script/Engine.Controller|GetPlayerState Target)))
  (Variables|/bomber-guys/Blueprints/Core/PS_BomberGuys.PS_BomberGuys_C|SetPlayerName _asps_bomber_guys PlayerName))

(event Custom|PawnEnemyKillFunction
  (Default|UpdatePlayersInfo (Variables|Default|GetUMG_DebugWidget)))

(event Custom|SpawnBonb
  (bind _returnvalue (Transformation|GetActorTransform))
  (bind _returnvalue_2 (Class|KismetMathLibrary|VectorSnappedtoGrid (.location _returnvalue) 1e+02))
  ;[1 0.586 0.1692 0.518] Spawn Bomb
  (if (Variables|Bomb|GetCanSpawnBomb) ; чтобы нельзя заспаунить больше бомб чем твой лимит
    (Variables|Bomb|SetcanSpawnHere true)
    (bind _outactors (Actor|GetAllActorsOfClass "/bomber-guys/Blueprints/Bomb/BP_Bomb.BP_Bomb_C"))
    (for _array_element _outactors
      (if (Utilities|Operators|EqualEqual (Transformation|GetActorLocation _array_element) _returnvalue_2 0.0)
        (Variables|Bomb|SetcanSpawnHere false)))
    (if (Variables|Bomb|GetcanSpawnHere) ; нельзя заспаунить бомбу одну в другой
      (Utilities|FlowControl|DoN (Variables|Bonuses|GetNBomb) :!label _label
        (:Exit
          (Utilities|SoundSpawnBomb)
          (Game|SpawnActorfromClass "/bomber-guys/Blueprints/Bomb/BP_Bomb.BP_Bomb_C" (Math|Transform|MakeTransform _returnvalue_2 "0, 0, 0" "0.800000,0.800000,0.800000") "Undefined" "MultiplyWithRoot" 0 (Variables|Bonuses|GetLengthOfFire) (Variables|Default|GetMaterial%20Bomb) (Variables|Bonuses|GetBombTime) self)
          ;[1 1 1] Время доСпавна бомбы
          (Utilities|FlowControl|Delay (Variables|Bonuses|GetBombTime))
          (goto _label Reset))))))

(event Custom|M_SpawnBomb
  ;[1 0.586 0.1692 0.518] Spawn Bomb
  ;;[1 0.9478 0.1968] Репликация спавн снаряда
  (if (not (Pawn|IsLocallyControlled))
    (CallFunction|SpawnBonb)))

(event Custom|S_SpawnBomb
  ;[1 0.586 0.1692 0.518] Spawn Bomb
  ;;[1 0.9478 0.1968] Репликация спавн снаряда
  (CallFunction|MSpawnBomb))

(event Custom|S_LengthOfFire++
  ;[0.9968 1 0.2442] Репликация длина волны
  (Variables|Bonuses|SetLengthOfFire (Math|Float|Clamp(Float) (+ (Variables|Bonuses|GetLengthOfFire) 1.0) 0.0 5.0)))

(event Custom|Kill
  (params (PC%20Ref :type Controller%20Object%20Reference))
  ;[1 0 0.12] Destroy and respawn character
  (Networking|SwitchHasAuthority
    (:Authority
      (bind _asgm_bomber_guys_base (Utilities|Casting|CastToGM_BomberGuysBase (Game|GetGameMode)))
      (Utilities|PlayDeathSound)
      (Default|GMRespawn _asgm_bomber_guys_base PC%20Ref))))

(event Custom|Bomb++
  ;[1 0.586 0.1692 0.518] Spawn Bomb
  (Variables|Bonuses|SetNBomb (+ (Variables|Bonuses|GetNBomb) 1)))

(event Custom|S_SetHeroStyle
  (params (Player%20EnumBP :type Enum_Color%20Enum :default "NewEnumerator0"))
  ;[1 0.9373 0.0697] Character color change
  (Variables|Default|SetPlayer%20EnumBP Player%20EnumBP))

(event Input|EnhancedActionEvents|EnhancedInputActionAI_Axis
  (params (ActionValue :type Vector%202D%20Structure) (ElapsedSeconds :type Float%20%28double-precision%29) (TriggeredSeconds :type Float%20%28double-precision%29) (InputAction :type Input%20Action%20Object%20Reference :default "/bomber-guys/Blueprints/Input/Actions/AI_Axis.AI_Axis"))
  ;[1 0.7353 0 0] Обзор
  (Pawn|Input|AddControllerYawInput (.x ActionValue))
  (Pawn|Input|AddControllerPitchInput (.y ActionValue)))

(event Input|EnhancedActionEvents|EnhancedInputActionAI_MoveUpDownL_R
  (params (ActionValue :type Vector%202D%20Structure) (ElapsedSeconds :type Float%20%28double-precision%29) (TriggeredSeconds :type Float%20%28double-precision%29) (InputAction :type Input%20Action%20Object%20Reference :default "/bomber-guys/Blueprints/Input/Actions/AI_MoveUpDownL_R.AI_MoveUpDownL_R"))
  (bind _returnvalue (Game|GetPlayerController 1))
  (bind _returnvalue_2 (Pawn|GetControlledPawn _returnvalue))
  ;[1 0.9196 0 0.099] Local character 2
  (Pawn|Input|AddMovementInput _returnvalue_2 "0.000000,1.000000,0.000000" (.x ActionValue) false)
  (Pawn|Input|AddMovementInput _returnvalue_2 "1.000000,0.000000,0.000000" (.y ActionValue) false))

(event Input|EnhancedActionEvents|EnhancedInputActionAI_Move
  (params (ActionValue :type Vector%202D%20Structure) (ElapsedSeconds :type Float%20%28double-precision%29) (TriggeredSeconds :type Float%20%28double-precision%29) (InputAction :type Input%20Action%20Object%20Reference :default "/bomber-guys/Blueprints/Input/Actions/AI_Move.AI_Move"))
  (bind _bodycamera (Variables|Default|GetBodyCamera))
  (bind _returnvalue (Math|Vector|GetRightVector _bodycamera))
  ;[0.6558 1 0.1521] Смена режима камеры
  ;;[0 1 0.168] Режим от 1 лица
  (if (not (Variables|Default|GetMove_n))
    (Pawn|Input|AddMovementInput (Math|Vector|MakeVector (.x _returnvalue) (.y _returnvalue) 0.0) (.x ActionValue) false)
    (Pawn|Input|AddMovementInput (Math|Vector|GetForwardVector _bodycamera) (.y ActionValue) false)))

(event Input|EnhancedActionEvents|EnhancedInputActionAI_Move
  (params (ActionValue :type Vector%202D%20Structure) (ElapsedSeconds :type Float%20%28double-precision%29) (TriggeredSeconds :type Float%20%28double-precision%29) (InputAction :type Input%20Action%20Object%20Reference :default "/bomber-guys/Blueprints/Input/Actions/AI_Move.AI_Move"))
  (bind _inversmove (Variables|Bonuses|GetInversMove))
  ;[1 0.8462 0 0.34] Player1 movement
  (if (Variables|Default|GetMove_n)
    (Pawn|Input|AddMovementInput (Math|Vector|MakeVector 0.0 _inversmove 0.0) (.x ActionValue) false)
    (Pawn|Input|AddMovementInput (Math|Vector|MakeVector _inversmove 0.0 0.0) (.y ActionValue) false)))

(event Input|EnhancedActionEvents|EnhancedInputActionIA_PauseGame
  (params (ActionValue :type Boolean) (ElapsedSeconds :type Float%20%28double-precision%29) (TriggeredSeconds :type Float%20%28double-precision%29) (InputAction :type Input%20Action%20Object%20Reference :default "/bomber-guys/Blueprints/Input/Actions/IA_PauseGame.IA_PauseGame"))
  ;[0.1431 1 0.04388] Pause game
  (:Started
    (if (Variables|Menu|GetPause)
      (Variables|Menu|SetPause false)
      (Widget|RemovefromParent (stale _returnvalue))
      (Game|SetGamePaused false)
      (else
        (Variables|Menu|SetPause true)
        (bind _returnvalue (UserInterface|CreateWidget "/bomber-guys/Blueprints/Pause/UMG_PauseGame.UMG_PauseGame_C" (Game|GetPlayerController 0)))
        (UserInterface|Viewport|AddtoViewport _returnvalue 0)
        (Game|SetGamePaused true)))))

(event EventBeginPlay
  (bind _returnvalue (Game|GetPlayerController 0))
  (Utilities|FlowControl|Sequence
    (:then_0
      (bind _outactors (Actor|GetAllActorswithTag "MainCamera"))
      (bind _asbp_game_camera (Utilities|Casting|CastToBP_GameCamera (Utilities|Array|Get(acopy) _outactors)))
      (Transformation|SetWorldTransform (Variables|Camera|GetThirdPersonCamera) (Transformation|GetActorTransform _asbp_game_camera) false false))
    (:then_1
      (bind _returnvalue_2 (Game|GetCurrentLevelName true))
      (if (not (Utilities|Enum|Equal(Enum) _returnvalue_2 "MenuMap"))
        (Utilities|Casting|CastToPC_BomberGuys _returnvalue)
        (Utilities|IsValid _returnvalue
          (:Is%20Valid
            (Input|SetInputModeGameOnly _returnvalue false)
            (Variables|/Script/Engine.PlayerController|SetbShowMouseCursor _returnvalue true)
            (Utilities|IsValid (Variables|Default|GetUMG_DebugWidget)
              (:Is%20Valid
                (Widget|RemovefromParent (Variables|Default|GetUMG_DebugWidget)))
              (:Is%20Not%20Valid
                _))
            (bind _returnvalue_3 (UserInterface|CreateWidget "/bomber-guys/Blueprints/GameplayWidgets/UMG_Debug.UMG_Debug_C" (Game|GetPlayerController 0)))
            (bind _output_get (Variables|Default|SetUMG_DebugWidget _returnvalue_3))
            (Utilities|IsValid _output_get
              (:Is%20Valid
                (UserInterface|Viewport|AddtoViewport _output_get 0)))))))
    (:then_2
      (Utilities|FlowControl|Sequence
        (:then_0
          ;[1 0.9373 0.0697] Character color change
          (bind _asgi_bomber_guys (Utilities|Casting|CastToGI_BomberGuys (Game|GetGameInstance)))
          (CallFunction|SSetHeroStyle (Variables|/bomber-guys/Blueprints/Core/GI_BomberGuys.GI_BomberGuys_C|GetPlayerEnum _asgi_bomber_guys)))
        (:then_1
          (bind _asgi_bomber_guys_2 (Utilities|Casting|CastToGI_BomberGuys (Game|GetGameInstance)))
          (Utilities|FlowControl|Sequence
            (:then_0
              (CallFunction|SSetPlayerNameinPS (Variables|/bomber-guys/Blueprints/Core/GI_BomberGuys.GI_BomberGuys_C|GetPlayerName _asgi_bomber_guys_2) (Game|GetPlayerController 0)))
            (:then_1
              (bind _asgs_bomber_guys (Utilities|Casting|CastToGS_BomberGuys (Game|GetGameState)))
              (Utilities|FlowControl|Delay 2.0) ; TODO Change to rep notify
              (for (_array_element _array_index) (Variables|/Script/Engine.GameStateBase|GetPlayerArray _asgs_bomber_guys)
                (bind _asps_bomber_guys (Utilities|Casting|CastToPS_BomberGuys _array_element))
                (Development|PrintString (Utilities|String|Append (Utilities|String|ToString(Integer) _array_index) "" (Variables|/bomber-guys/Blueprints/Core/PS_BomberGuys.PS_BomberGuys_C|GetPlayerName _asps_bomber_guys)))
                (Default|UpdatePlayersInfo (Variables|Default|GetUMG_DebugWidget))))))))))

(event Input|KeyboardEvents|SpaceBar
  (params (Key :type Key%20Structure :default "None"))
  (bind _returnvalue (Game|GetPlayerController 1))
  (bind _returnvalue_2 (Pawn|GetControlledPawn _returnvalue))
  ;[1 0.9196 0 0.099] Local character 2
  (:Pressed
    (Utilities|IsValid _returnvalue_2
      (:Is%20Valid
        (bind _asbp_bomber_guy (Utilities|Casting|CastToBP_BomberGuy _returnvalue_2))
        (Utilities|IsValid _asbp_bomber_guy
          (:Is%20Valid
            (CallFunction|SpawnBonb _asbp_bomber_guy)))))))

(event Input|KeyboardEvents|F
  (params (Key :type Key%20Structure :default "None"))
  ;[0.6558 1 0.1521] Смена режима камеры
  (:Pressed
    (Utilities|FlowControl|FlipFlop
      (:A
        (Variables|Default|SetMove_n false)
        (Components|Activation|Deactivate (Variables|Camera|GetThirdPersonCamera))
        (Components|Activation|Activate (Variables|Default|GetBodyCamera) true)
        (Variables|/Script/Engine.PlayerController|SetbShowMouseCursor (Game|GetPlayerController 0) false)
        (Variables|Default|SetbUseControllerRotationYaw true))
      (:B
        (Variables|Default|SetMove_n true)
        (Components|Activation|Deactivate (Variables|Default|GetBodyCamera))
        (Components|Activation|Activate (Variables|Camera|GetThirdPersonCamera) true)
        (Variables|/Script/Engine.PlayerController|SetbShowMouseCursor (Game|GetPlayerController 0) false)
        (Variables|Default|SetbUseControllerRotationYaw false)))))

(event Input|KeyboardEvents|LeftShift
  (params (Key :type Key%20Structure :default "None"))
  ;[1 0.586 0.1692 0.518] Spawn Bomb
  ;;[1 0.9478 0.1968] Репликация спавн снаряда
  (:Pressed
    (CallFunction|SpawnBonb)
    (Networking|SwitchHasAuthority
      (:Authority
        (CallFunction|MSpawnBomb))
      (:Remote
        (CallFunction|SSpawnBomb)))))

(event Input|KeyboardEvents|Y
  (params (Key :type Key%20Structure :default "None"))
  (:Pressed
    (bind _asgs_bomber_guys (Utilities|Casting|CastToGS_BomberGuys (Game|GetGameState)))
    (for (_array_element _array_index) (Variables|/Script/Engine.GameStateBase|GetPlayerArray _asgs_bomber_guys)
      (bind _asps_bomber_guys (Utilities|Casting|CastToPS_BomberGuys _array_element))
      (Development|PrintString (Utilities|String|Append (Utilities|String|ToString(Integer) _array_index) "" (Variables|/bomber-guys/Blueprints/Core/PS_BomberGuys.PS_BomberGuys_C|GetPlayerName _asps_bomber_guys) "kills; " " " (Utilities|String|ToString(Integer) (Variables|/bomber-guys/Blueprints/Core/PS_BomberGuys.PS_BomberGuys_C|GetnumberOfKills _asps_bomber_guys)))))))

(event Input|KeyboardEvents|T
  (params (Key :type Key%20Structure :default "None"))
  (:Pressed
    (Utilities|Casting|CastToGS_BomberGuys (Game|GetGameState))))

(event Input|KeyboardEvents|J
  (params (Key :type Key%20Structure :default "None"))
  (:Pressed
    (bind _asps_bomber_guys (Utilities|Casting|CastToPS_BomberGuys (Variables|/Script/Engine.Controller|GetPlayerState (Game|GetPlayerController 0))))
    (Development|PrintString (Utilities|String|Append (Variables|/bomber-guys/Blueprints/Core/PS_BomberGuys.PS_BomberGuys_C|GetPlayerName _asps_bomber_guys) "--" (Utilities|String|ToString(Integer) (Variables|/bomber-guys/Blueprints/Core/PS_BomberGuys.PS_BomberGuys_C|GetnumberOfKills _asps_bomber_guys))))))

(fn ConstructionScript
  (Components|SkinnedMesh|HideBonebyName (Variables|Character|GetMesh) "None" "PBO_None"))

(fn OnRepPlayerEnumBP
  (switch Utilities|FlowControl|Switch|SwitchonEnum_Color (Variables|Default|GetPlayer%20EnumBP)
    (:NewEnumerator0
      (Components|SkeletalMesh|SetSkeletalMeshAsset (Variables|Character|GetMesh) "/bomber-guys/Static/BomberGuyColors/robot_White.robot_White")
      (Variables|Default|SetMaterial%20Bomb "/bomber-guys/Static/BomberGuyColors/Collor/Mi_Write.Mi_Write")
      (Variables|Default|SetFootprintColor "(R=1.000000,G=1.000000,B=1.000000,A=1.000000)"))
    (:NewEnumerator1
      (Components|SkeletalMesh|SetSkeletalMeshAsset (Variables|Character|GetMesh) "/bomber-guys/Static/BomberGuyColors/robot_Black.robot_Black")
      (Variables|Default|SetMaterial%20Bomb "/bomber-guys/Static/BomberGuyColors/Collor/Mi_BlackRobot.Mi_BlackRobot")
      (Variables|Default|SetFootprintColor "(R=0.000000,G=0.000000,B=0.000000,A=1.000000)"))
    (:NewEnumerator2
      (Components|SkeletalMesh|SetSkeletalMeshAsset (Variables|Character|GetMesh) "/bomber-guys/Static/BomberGuyColors/robot_Red.robot_Red")
      (Variables|Default|SetMaterial%20Bomb "/bomber-guys/Static/BomberGuyColors/Collor/Mi_Red.Mi_Red")
      (Variables|Default|SetFootprintColor "(R=1.000000,G=0.000000,B=0.000000,A=1.000000)"))
    (:NewEnumerator3
      (Components|SkeletalMesh|SetSkeletalMeshAsset (Variables|Character|GetMesh) "/bomber-guys/Static/BomberGuyColors/robot_Blue.robot_Blue")
      (Variables|Default|SetMaterial%20Bomb "/bomber-guys/Static/BomberGuyColors/Collor/Mi_Blue.Mi_Blue")
      (Variables|Default|SetFootprintColor "(R=0.000630,G=0.000000,B=1.000000,A=1.000000)"))
    (:NewEnumerator4
      (Components|SkeletalMesh|SetSkeletalMeshAsset (Variables|Character|GetMesh) "/bomber-guys/Static/BomberGuyColors/robot_Green.robot_Green")
      (Variables|Default|SetMaterial%20Bomb "/bomber-guys/Static/BomberGuyColors/Collor/Mi_Green.Mi_Green")
      (Variables|Default|SetFootprintColor "(R=0.000000,G=1.000000,B=0.000000,A=1.000000)"))
    (:NewEnumerator5
      (Components|SkeletalMesh|SetSkeletalMeshAsset (Variables|Character|GetMesh) "/bomber-guys/Static/BomberGuyColors/robot__Yellow.robot__Yellow")
      (Variables|Default|SetMaterial%20Bomb "/bomber-guys/Static/BomberGuyColors/Collor/Mi_Jelow.Mi_Jelow")
      (Variables|Default|SetFootprintColor "(R=1.000000,G=1.000000,B=0.000000,A=1.000000)"))
    (:NewEnumerator6
      (Components|SkeletalMesh|SetSkeletalMeshAsset (Variables|Character|GetMesh) "/bomber-guys/Static/BomberGuyColors/robot_LightBlue.robot_LightBlue")
      (Variables|Default|SetMaterial%20Bomb "/bomber-guys/Static/BomberGuyColors/Collor/Mi_LightBlue.Mi_LightBlue")
      (Variables|Default|SetFootprintColor "(R=0.223958,G=1.000000,B=0.966716,A=1.000000)"))
    (:NewEnumerator7
      (Components|SkeletalMesh|SetSkeletalMeshAsset (Variables|Character|GetMesh) "/bomber-guys/Static/BomberGuyColors/robot_Pink.robot_Pink")
      (Variables|Default|SetMaterial%20Bomb "/bomber-guys/Static/BomberGuyColors/Collor/Mi_Pink.Mi_Pink")
      (Variables|Default|SetFootprintColor "(R=0.904661,G=0.174647,B=0.830770,A=1.000000)"))
    (:NewEnumerator8
      (Components|SkeletalMesh|SetSkeletalMeshAsset (Variables|Character|GetMesh) "/bomber-guys/Static/BomberGuyColors/robot_Orange.robot_Orange")
      (Variables|Default|SetMaterial%20Bomb "/bomber-guys/Static/BomberGuyColors/Collor/Mi_Orange.Mi_Orange")
      (Variables|Default|SetFootprintColor "(R=1.000000,G=0.323075,B=0.000000,A=1.000000)"))
    (:NewEnumerator9
      (Components|SkeletalMesh|SetSkeletalMeshAsset (Variables|Character|GetMesh) "/bomber-guys/Static/BomberGuyColors/robot_Violet.robot_Violet")
      (Variables|Default|SetMaterial%20Bomb "/bomber-guys/Static/BomberGuyColors/Collor/Mi_Violet.Mi_Violet")
      (Variables|Default|SetFootprintColor "(R=0.153511,G=0.029313,B=0.708333,A=1.000000)"))))